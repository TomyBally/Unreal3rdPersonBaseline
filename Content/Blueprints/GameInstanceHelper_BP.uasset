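; GameInstanceHelper_BP is a helper that runs a five-second countdown stored in the game instance.
; On BeginPlay it casts and caches GameInstance_BP, sets its Timer to the starting value and prints a startup message.
; Tick feeds a one-second Delay, which ignores calls while pending, so Timer drops by one roughly each second until it reaches zero.
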(event EventBeginPlay
  (bind _asgame_instance_bp (Utilities|Casting|CastToGameInstance_BP (Game|GetGameInstance)))
  (bind _output_get (Variables|Default|SetGI_Instance _asgame_instance_bp))
  (Variables|/Game/Blueprints/GameInstance_BP.GameInstance_BP_C|SetTimer _output_get 5)
  (Development|PrintString "Helper started"))

(event Collision|EventActorBeginOverlap
  (params (OtherActor :type Actor%20Object%20Reference)))

(event EventTick
  (params (DeltaSeconds :type Float%20%28single-precision%29))
  (bind _gi_instance (Variables|Default|GetGI_Instance))
  (Utilities|FlowControl|Sequence
    (:then_0
      (Utilities|FlowControl|Delay 1.0)
      ;[1 1 1] Update Timer
      (if (> (Variables|/Game/Blueprints/GameInstance_BP.GameInstance_BP_C|GetTimer _gi_instance) 0)
        (bind _result (Math|Integer|DecrementInt (Variables|/Game/Blueprints/GameInstance_BP.GameInstance_BP_C|GetTimer _gi_instance))
          (:%20%20
            (Variables|/Game/Blueprints/GameInstance_BP.GameInstance_BP_C|SetTimer _gi_instance _result)))))))

(fn ConstructionScript)