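; Pickup actor that the ThirdPersonCharacter collects by overlapping it, triggering the character's PickupEvent with a fixed amount.
; An IsUnused flag, cleared once the cast succeeds, limits it to one collection and prints a hit message.
; The ScaleDown timeline then scales the actor from its starting scale and destroys it when finished.
; BeginPlay caches the first UI_BP widget, though nothing here uses it.
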(event EventBeginPlay
  (bind _foundwidgets (Widget|GetAllWidgetsOfClass "/Game/UI_BP.UI_BP_C" true))
  (Variables|Default|SetUI_Widget (Utilities|Array|Get(acopy) _foundwidgets)))

(event Collision|EventActorBeginOverlap
  (params (OtherActor :type Actor%20Object%20Reference))
  (if (Variables|Default|GetisUnused)
    (bind _asthird_person_character (Utilities|Casting|CastToThirdPersonCharacter OtherActor))
    (Variables|Default|SetisUnused false)
    (Development|PrintString (Utilities|String|ToString(Text) (Utilities|Text|FormatText "Hit {Character}" (Utilities|Text|ToText(String) (Utilities|GetDisplayName _asthird_person_character)))))
    (Default|PickupEvent _asthird_person_character 10)
    (bind _output_get (Variables|Default|SetStartValue (Class|Actor|GetActorRelativeScale3D)))
    (bind _time (Timeline|ScaleDown Play)
      (:Update
        (Transformation|SetActorScale3D (* _output_get _time)))
      (:Finished
        (Actor|DestroyActor)))))

(event EventTick
  (params (DeltaSeconds :type Float%20%28single-precision%29)))

(fn ConstructionScript)